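; Saber creature character Blueprint that adds a meteor barrage attack and scaled resource harvesting.
; Attack index 1 triggers the FireProjectile ROS event, which uses nested Sequences and Delays to stagger eight ProjMeteor spawns.
; Each meteor spawns at its own Box component's transform and launches along that box's forward vector.
; The harvesting override multiplies quantities for resource classes matched in ResourceTypesToScale by their paired ResourceTypeScales entry.
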(event Custom|FireProjectile_ROS
  (bind _box1 (Variables|Default|GetBox1))
  (bind _box2 (Variables|Default|GetBox2))
  (bind _box3 (Variables|Default|GetBox3))
  (bind _box4 (Variables|Default|GetBox4))
  (bind _box5 (Variables|Default|GetBox5))
  (bind _box6 (Variables|Default|GetBox6))
  (bind _box7 (Variables|Default|GetBox7))
  (bind _box8 (Variables|Default|GetBox8))
  (bind _returnvalue (Transformation|GetWorldRotation _box8))
  (bind _returnvalue_2 (Transformation|GetWorldRotation _box2))
  (bind _returnvalue_3 (Transformation|GetWorldRotation _box3))
  (bind _returnvalue_4 (Transformation|GetWorldRotation _box4))
  (bind _returnvalue_5 (Transformation|GetWorldRotation _box1))
  (bind _returnvalue_6 (Transformation|GetWorldRotation _box5))
  (bind _returnvalue_7 (Transformation|GetWorldRotation _box6))
  (bind _returnvalue_8 (Transformation|GetWorldRotation _box7))
  ;[1 1 1] Meteor attack
  (Utilities|FlowControl|Sequence
    (:then_0
      (Utilities|FlowControl|Delay 0.2)
      (Utilities|FlowControl|Sequence
        (:then_0
          (bind _returnvalue_9 (Game|SpawnActorfromClass "/Game/Mods/test/MeteorSaber/ProjMeteor.ProjMeteor_C" (Math|Transform|MakeTransform (Transformation|GetWorldLocation _box1) _returnvalue_5) false 0))
          (Class|ShooterProjectile|BPInitVelocity _returnvalue_9 (Math|Vector|GetForwardVector _returnvalue_5)))
        (:then_1
          (Utilities|FlowControl|Delay 0.6)
          (bind _returnvalue_10 (Game|SpawnActorfromClass "/Game/Mods/test/MeteorSaber/ProjMeteor.ProjMeteor_C" (Math|Transform|MakeTransform (Transformation|GetWorldLocation _box2) _returnvalue_2) false 0))
          (Class|ShooterProjectile|BPInitVelocity _returnvalue_10 (Math|Vector|GetForwardVector _returnvalue_2)))
        (:then_2
          (Utilities|FlowControl|Delay 1.0)
          (bind _returnvalue_11 (Game|SpawnActorfromClass "/Game/Mods/test/MeteorSaber/ProjMeteor.ProjMeteor_C" (Math|Transform|MakeTransform (Transformation|GetWorldLocation _box3) _returnvalue_3) false 0))
          (Class|ShooterProjectile|BPInitVelocity _returnvalue_11 (Math|Vector|GetForwardVector _returnvalue_3)))
        (:then_3
          (Utilities|FlowControl|Delay 1.5)
          (bind _returnvalue_12 (Game|SpawnActorfromClass "/Game/Mods/test/MeteorSaber/ProjMeteor.ProjMeteor_C" (Math|Transform|MakeTransform (Transformation|GetWorldLocation _box4) _returnvalue_4) false 0))
          (Class|ShooterProjectile|BPInitVelocity _returnvalue_12 (Math|Vector|GetForwardVector _returnvalue_4)))))
    (:then_1
      (Utilities|FlowControl|Delay 1.0)
      (Utilities|FlowControl|Sequence
        (:then_0
          (Utilities|FlowControl|Delay 0.7)
          (bind _returnvalue_13 (Game|SpawnActorfromClass "/Game/Mods/test/MeteorSaber/ProjMeteor.ProjMeteor_C" (Math|Transform|MakeTransform (Transformation|GetWorldLocation _box5) _returnvalue_6) false 0))
          (Class|ShooterProjectile|BPInitVelocity _returnvalue_13 (Math|Vector|GetForwardVector _returnvalue_6)))
        (:then_1
          (Utilities|FlowControl|Delay 0.5)
          (bind _returnvalue_14 (Game|SpawnActorfromClass "/Game/Mods/test/MeteorSaber/ProjMeteor.ProjMeteor_C" (Math|Transform|MakeTransform (Transformation|GetWorldLocation _box6) _returnvalue_7) false 0))
          (Class|ShooterProjectile|BPInitVelocity _returnvalue_14 (Math|Vector|GetForwardVector _returnvalue_7)))
        (:then_2
          (Utilities|FlowControl|Delay 1.2)
          (bind _returnvalue_15 (Game|SpawnActorfromClass "/Game/Mods/test/MeteorSaber/ProjMeteor.ProjMeteor_C" (Math|Transform|MakeTransform (Transformation|GetWorldLocation _box7) _returnvalue_8) false 0))
          (Class|ShooterProjectile|BPInitVelocity _returnvalue_15 (Math|Vector|GetForwardVector _returnvalue_8)))
        (:then_3
          (Utilities|FlowControl|Delay 1.6)
          (bind _returnvalue_16 (Game|SpawnActorfromClass "/Game/Mods/test/MeteorSaber/ProjMeteor.ProjMeteor_C" (Math|Transform|MakeTransform (Transformation|GetWorldLocation _box8) _returnvalue) false 0))
          (Class|ShooterProjectile|BPInitVelocity _returnvalue_16 (Math|Vector|GetForwardVector _returnvalue)))))))

(fn ConstructionScript
  (|CallParentFunction))

(fn BPModifyHarvestingQuantity
  (params (originalQuantity :type Float%20%28single-precision%29) (resourceSelected :type Primal%20Item%20Class%20Reference))
  (LocalVariables|SetAmountOut originalQuantity)
  (Utilities|FlowControl|Sequence
    (:then_0
      (bind _returnvalue (Class|VictoryCore|IsChildOfClasses resourceSelected (Variables|Default|GetResourceTypesToScale)))
      (if (!= _returnvalue -1)
        (LocalVariables|SetAmountOut (* (LocalVariables|GetAmountOut) (Utilities|Array|Get(acopy) (Variables|Default|GetResourceTypeScales) _returnvalue)))))
    (:then_1
      (return (LocalVariables|GetAmountOut)))))

(fn BPDoAttack
  (params (AttackIndex :type Integer))
  (if (== AttackIndex 1)
    (CallFunction|FireProjectileROS)))